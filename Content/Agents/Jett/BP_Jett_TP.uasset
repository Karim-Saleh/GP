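; Third-person Blueprint for the Jett agent, holding test logic for attaching and dropping a Vandal weapon.
; Interact snaps Vandal onto the PrimaryWeapon child actor component, then snaps that component to the Vandal socket on FPMesh.
; Drop Item stores the component's child actor as Vandal and detaches it, keeping its world transform.
; BeginPlay is empty, the overlap event is disabled, and Tick and construction only call the parent.
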(event `self.ReceiveBeginPlay`)

(event `self.ReceiveTick`
  (params (DeltaSeconds :type "Float (single-precision)"))
  (`parent.ReceiveTick` DeltaSeconds))

(event `InputAction|Interact`
  (params (Key :type "Key Structure"))
  (bind _primary_weapon (`self.Primary Weapon`))
  ;[1 1 1] Test Weapon Attachment
  (:`Pressed`
    (`self.K2_AttachToComponent` (`self.vandal`) _primary_weapon "None" "SnapToTarget" "SnapToTarget" "SnapToTarget" true)
    (`SceneComponent.K2_AttachToComponent` _primary_weapon (`self.FP Mesh`) "Vandal_Socket" "SnapToTarget" "SnapToTarget" "SnapToTarget" true)))

(event `InputAction|Drop Item`
  (params (Key :type "Key Structure"))
  (bind _childactor (`ChildActorComponent.ChildActor` (`self.Primary Weapon`)))
  ;[1 1 1] Test Weapon Attachment
  (:`Pressed`
    (set `self.vandal` _childactor)
    (`self.K2_DetachFromActor` _childactor "KeepWorld" "KeepWorld" "KeepWorld")))

(fn `UserConstructionScript`
  (`parent.UserConstructionScript`))