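; Yoru agent Blueprint that extends a parent class and holds test logic for weapon attachment.
; Interact snaps the Vandal onto the PrimaryWeapon child actor component, then snaps that component to the first-person mesh's Vandal socket.
; Drop Item stores the child actor as Vandal and detaches it, keeping its world transform.
; CheckIfPrimary always returns true, and the point damage handler is empty and never bound.
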(event `self.ReceiveBeginPlay`)

(event `self.ReceiveTick`
  (params (DeltaSeconds :type "Float (single-precision)"))
  (`parent.ReceiveTick` DeltaSeconds))

(event `InputAction|Interact`
  (params (Key :type "Key Structure"))
  (bind _primary_weapon (`self.Primary Weapon`))
  ;[1 1 1] Test Weapon Attachment
  (:`Pressed`
    (`self.K2_AttachToComponent` (`self.vandal`) _primary_weapon "None" "SnapToTarget" "SnapToTarget" "SnapToTarget" true)
    (`SceneComponent.K2_AttachToComponent` _primary_weapon (`self.FP Mesh`) "Vandal_Socket" "SnapToTarget" "SnapToTarget" "SnapToTarget" true)))

(event `InputAction|Drop Item`
  (params (Key :type "Key Structure"))
  (bind _childactor (`ChildActorComponent.ChildActor` (`self.Primary Weapon`)))
  ;[1 1 1] Test Weapon Attachment
  (:`Pressed`
    (set `self.vandal` _childactor)
    (`self.K2_DetachFromActor` _childactor "KeepWorld" "KeepWorld" "KeepWorld")))

(event `OnTakePointDamage_Event` :!signature `self.OnTakePointDamage`
  (params (DamagedActor :type "Actor Object Reference") (Damage :type "Float (single-precision)") (InstigatedBy :type "Controller Object Reference") (HitLocation :type "Vector Structure") (FHitComponent :type "PrimitiveComponent Object Reference") (BoneName :type Name) (ShotFromDirection :type "Vector Structure") (DamageType :type "DamageType Object Reference") (DamageCauser :type "Actor Object Reference")))

(fn `Check if Primary`
  (returns (`Is Primary` :type Boolean))
  (return true))

(fn `UserConstructionScript`
  (`parent.UserConstructionScript`))