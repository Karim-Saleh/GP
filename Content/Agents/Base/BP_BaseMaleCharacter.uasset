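; Base male agent character Blueprint that handles first-person reload animations and damage to armor and health.
; ReloadAnimation plays a montage behind a DoOnce gate; for the Vandal, montage notifies toggle a temporary magazine mesh, which is also hidden on interrupt.
; PointDamage lazily creates a blood-screen widget, plays its hit animation, then drains armor before health.
; Death only zeroes health and prints a debug message.
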(event `self.ReceiveBeginPlay`)

(event `self.ReceiveTick`
  (params (DeltaSeconds :type "Float (single-precision)")))

(event `/Game/Agents/Base/Interfaces/CharacterAnimationsInterface.Reload Animation`
  (params (Motage :type "AnimMontage Object Reference") (Vandal :type Boolean))
  (bind _vandal_temp_mag (`self.Vandal Temp Mag`))
  ;[0.1747 0.6942 0.7802 1 30] Reloading Animations
  (`/Engine/EditorBlueprintResources/StandardMacros.DoOnce` false :!label _label
    (:`Completed`
      (bind _notifyname (`|PlayMontage` (`self.FP Mesh`) Motage (`self.Montages Play Rate`))
        (:`OnCompleted`
          (goto _label :!via `Reset`))
        (:`OnInterrupted`
          (`SceneComponent.SetVisibility` _vandal_temp_mag false true :!label _label_2)
          (goto _label :!via `Reset`))
        (:`OnNotifyBegin`
          (if Vandal
            (if (== _notifyname "Start")
              (`SceneComponent.SetVisibility` _vandal_temp_mag true true)
              (else
                (goto _label_2)))))))))

(event `self.ReceivePointDamage`
  (params (Damage :type "Float (single-precision)") (DamageType :type "DamageType Object Reference") (HitLocation :type "Vector Structure") (HitNormal :type "Vector Structure") (HitComponent :type "PrimitiveComponent Object Reference") (BoneName :type Name) (ShotFromDirection :type "Vector Structure") (InstigatedBy :type "Controller Object Reference") (DamageCauser :type "Actor Object Reference") (HitInfo :type "HitResult Structure (by ref)"))
  ;[0.2386 0.3867 1] Damage System
  (`self.BloodWidget`
    (:`then`
      _)
    (:`else`
      (bind _returnvalue (`|CreateWidget` "/Game/UI/Widgets/BloodScreen_wd.BloodScreen_wd_C" (`GameplayStatics.GetPlayerController` 0)))
      (bind _output_get (set `self.BloodWidget` _returnvalue))
      (`UserWidget.AddToViewport` _output_get 0)))
  (`/Game/UI/Widgets/BloodScreen_wd.PlayHitAnimation` (`self.BloodWidget`))
  (bind _output_get_2 (set `self.tempdamage` Damage))
  (bind _output_get_3 (set `self.total Hp ` (+ (`self.Armor`) (`self.Health`))))
  (if (>= Damage _output_get_3)
    (set `self.Health` 0.0)
    (`KismetSystemLibrary.PrintString` "died" true true (struct :`R` 1.0 :`G` 0.075233 :`A` 1.0))
    (elif (>= (`self.Armor`) _output_get_2)
      (set `self.Armor` (- (`self.Armor`) (`self.tempdamage`)))
      (set `self.total Hp ` (+ (`self.Armor`) (`self.Health`)))
      (`KismetSystemLibrary.PrintString` (`KismetStringLibrary.Conv_DoubleToString` (`self.total Hp `)) true true (struct :`R` 0.148253 :`G` 1.0 :`A` 1.0))
      (else
        (bind _output_get_4 (set `self.tempdamage` (- (`self.tempdamage`) (`self.Armor`))))
        (set `self.Armor` 0.0)
        (bind _output_get_5 (set `self.Health` (- (`self.Health`) _output_get_4)))
        (`KismetSystemLibrary.PrintString` (`KismetStringLibrary.Conv_DoubleToString` _output_get_5) true true (struct :`R` 0.955192 :`G` 1.0 :`A` 1.0))))))

(fn `UserConstructionScript`)