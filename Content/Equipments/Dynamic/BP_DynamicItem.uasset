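; BP_DynamicItem is an item actor that shows an interaction prompt while a player is in interaction range.
; On range entry it creates a text widget for that player's controller and attaches it through a runtime-added, screen-space widget component without collision.
; On range exit it destroys that component.
; Two functions supply the prompt text and attach point, defaulting to "interact" and the scene root.
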(event `/Game/Equipments/Dynamic/interactionInterface.onInteractionRangeEntered`
  (params (player :type "/Game/AnimStarterPack/Ue4ASP_Character Object Reference"))
  (`self.interactionWidgetComponent`
    (:`then`)
    (:`else`
      (bind _returnvalue (`|GenericCreateObject` (cast `PlayerController` (`Pawn.GetController` player) :!pure true) "/Game/UI/Widgets/interactionWidget.interactionWidget_C" (`self.Get Interaction Text`)))
      (bind _returnvalue_2 (`AddComponent|NODE_AddWidgetComponent-0`))
      (bind _output_get (set `self.interactionWidgetComponent` _returnvalue_2))
      (`WidgetComponent.SetWidget` _output_get _returnvalue)
      (`WidgetComponent.SetWidgetSpace` _output_get "Screen")
      (`WidgetComponent.SetDrawAtDesiredSize` _output_get true)
      (`PrimitiveComponent.SetCollisionEnabled` _output_get "NoCollision")
      (`SceneComponent.K2_AttachToComponent` _output_get (`self.geInteractionTextAttach`) "None" "SnapToTarget" "SnapToTarget" "SnapToTarget" true))))

(event `/Game/Equipments/Dynamic/interactionInterface.onInteractionRangeExited`
  (bind _interactionwidgetcomponent (`self.interactionWidgetComponent`)
    (:`then`
      (`ActorComponent.K2_DestroyComponent` _interactionwidgetcomponent))
    (:`else`)))

(fn `geInteractionTextAttach`
  (returns (attachComponent :type "SceneComponent Object Reference"))
  (return (`self.DefaultSceneRoot`)))

(fn `Get Interaction Text`
  (returns (text :type Text))
  (return "interact"))

(fn `UserConstructionScript`
  (`parent.UserConstructionScript`))