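; BP_Classic is the Classic pistol weapon, a child Blueprint that relies on its parent class for its behavior.
; It overrides Reload Anim & Sound to run the parent logic, then play the Classic reload animation once on the Weapon component.
; The event graph holds only disabled default events, and the construction script just calls the parent.
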(fn `Reload Anim & Sound`
  (params (`Character Mesh` :type "SkeletalMeshComponent Object Reference"))
  (`parent.Reload Anim & Sound` `Character Mesh`)
  (`SkeletalMeshComponent.PlayAnimation` (`self.Weapon`) "/Game/Equipments/Dynamic/Weapons/Pistols/Classic/AnimationPack/Classic_Reload_MO.Classic_Reload_MO" false))

(fn `UserConstructionScript`
  (`parent.UserConstructionScript`))