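; Weapon actor that handles hitscan firing, ammo tracking and reloading.
; Fire line-traces from the passed camera, applies head or body damage by hit bone, spawns muzzle effects and reports an AI noise event at the player pawn.
; Reload plays a montage behind a DoOnce, and UpdateAmmo refills the magazine from reserve on completion, using Abs arithmetic as a branchless clamp.
; Debug trace drawing and print strings remain active in Fire.
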(event `/Game/Equipments/Dynamic/WeaponAnimationInterface.Reload Animation`
  (`/Engine/EditorBlueprintResources/StandardMacros.DoOnce` false :!label _label
    (:`Completed`
      (set `self.IsReloading` true)
      (`|PlayMontage` (`self.Weapon`) (`self.Weapon Reload Montage`) 1.5
        (:`OnCompleted`
          (`self.Update Ammo`))
        (:`OnInterrupted`
          _))
      (set `self.IsReloading` false)
      (goto _label :!via `Reset`))))

(fn `Can Reload?`
  (returns (ReturnValue :type Boolean))
  (return (and (> (`self.Max Ammo`) 0) (< (`self.Current Ammo`) (`self.Magazine Size`)))))

(fn `Fire`
  (params (Camera :type "SceneComponent Object Reference") (Character :type "Character Object Reference"))
  (bind _returnvalue (`SceneComponent.K2_GetComponentLocation` Camera))
  (bind _returnvalue_2 (`GameplayStatics.GetPlayerPawn` 0))
  (bind _returnvalue_3 (`SceneComponent.GetSocketLocation` (`self.Weapon`) "Muzzle"))
  (bind _outhit (`KismetSystemLibrary.LineTraceSingle` _returnvalue (+ _returnvalue (* 10000.0 (`SceneComponent.GetForwardVector` Camera))) "TraceTypeQuery2" false (`|MakeArray` (`local.Character`) :!type "Actor Object Reference") "Persistent" true (struct :`R` 1.0 :`A` 1.0) (struct :`G` 1.0 :`A` 1.0) 2.0))
  (bind (_bblockinghit _binitialoverlap _time _distance _location _impactpoint _normal _impactnormal _physmat _hitactor _hitcomponent _hitbonename _bonename _hititem _elementindex _faceindex _tracestart) (`GameplayStatics.BreakHitResult` _outhit))
  (`GameplayStatics.ApplyPointDamage` _hitactor (`KismetMathLibrary.SelectFloat` (`self.HeadShotDamage`) (`self.BodyDamge`) (== _hitbonename "Head")) _tracestart _outhit)
  (`GameplayStatics.PlaySoundAtLocation` "/Game/Audio/GUN_FIRE-GoodSoundForYou-820112263.GUN_FIRE-GoodSoundForYou-820112263" _returnvalue_3 (struct) 1.0 1.0 0.0 null null null null)
  (`|SpawnActorFromClass` "/Game/Equipments/Dynamic/Weapons/Shared/BP_MuzzleFlash.BP_MuzzleFlash_C" (`KismetMathLibrary.MakeTransform` _returnvalue_3) "Undefined" "OverrideRootScale" null null)
  (`/Engine/EditorBlueprintResources/StandardMacros.DecrementInt` (`self.Current Ammo`)
    (:`  `
      (`KismetSystemLibrary.PrintString` (`KismetStringLibrary.Conv_NameToString` _hitbonename))
      (if (== _returnvalue_2 (`GameplayStatics.GetPlayerCharacter` 0))
        (`AISense_Hearing.ReportNoiseEvent` (`self.K2_GetActorLocation` _returnvalue_2) 1.0 _returnvalue_2)
        (`KismetSystemLibrary.PrintString` "produced sound")))))

(fn `Reload`
  (`/Game/Equipments/Dynamic/WeaponAnimationInterface.Reload Animation`))

(fn `Update Ammo`
  (locals (Temp :type Integer))
  (`|ExecutionSequence`
    (:`then_0`
      ;[1 1 1] Calculate Temp
      (set `local.Temp` (- (`self.Max Ammo`) (- (`self.Magazine Size`) (`self.Current Ammo`)))))
    (:`then_1`
      ;[1 1 1] Setting Current Ammo
      (set `self.Current Ammo` (+ (`self.Magazine Size`) (/ (- (`local.Temp`) (`KismetMathLibrary.Abs_Int` (`local.Temp`))) 2))))
    (:`then_2`
      ;[1 1 1] Setting Max Ammo
      (set `self.Max Ammo` (/ (+ (`local.Temp`) (`KismetMathLibrary.Abs_Int` (`local.Temp`))) 2)))))

(fn `UserConstructionScript`
  (`parent.UserConstructionScript`))